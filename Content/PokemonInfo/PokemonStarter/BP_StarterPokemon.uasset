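; Starter Pokémon pickup actor that offers its Pokémon to a player whose party is empty.
; A box overlap toggles input, letting debug key E scan the trainer party and open W_AcceptPokemon with UI-only input, switching movement to Swimming.
; RollforInfo, not called here, sets level 5 and gender once; its RandomInteger(1) roll always yields zero, so gender never varies.
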(event OnComponentBeginOverlap(Box)
  (params (OverlappedComponent :type Primitive%20Component%20Object%20Reference) (OtherActor :type Actor%20Object%20Reference) (OtherComp :type Primitive%20Component%20Object%20Reference) (OtherBodyIndex :type Integer) (bFromSweep :type Boolean) (SweepResult :type Hit%20Result%20Structure%20%28by%20ref%29))
  ;[0.05098 0.05098 0.05098] Set Overlap
  (bind _asbp_third_person_character (Utilities|Casting|CastToBP_ThirdPersonCharacter OtherActor))
  (Variables|Default|SetTPC%20Ref _asbp_third_person_character)
  (Input|EnableInput (Game|GetPlayerController 0)))

(event OnComponentEndOverlap(Box)
  (params (OverlappedComponent :type Primitive%20Component%20Object%20Reference) (OtherActor :type Actor%20Object%20Reference) (OtherComp :type Primitive%20Component%20Object%20Reference) (OtherBodyIndex :type Integer))
  ;[0.05098 0.05098 0.05098] Set Overlap
  (Utilities|Casting|CastToBP_ThirdPersonCharacter OtherActor)
  (Input|DisableInput (Game|GetPlayerController 0)))

(event Custom|Roll%20for%20Info
  ;[0.05098 0.05098 0.05098] Set Information Starter
  (Utilities|FlowControl|DoOnce false
    (:Completed
      (if (== (Math|Random|RandomInteger 1) 1)
        (Variables|Default|SetGender "NewEnumerator1")
        (else
          (Variables|Default|SetGender "NewEnumerator2")))
      (bind _structout (Utilities|Struct|SetmembersinFPokemonPartyInfo (Variables|Default|GetStarterPokemon) 5 false (Variables|Default|GetGender)))
      (Variables|Default|SetStarterPokemon _structout))))

(event Input|KeyboardEvents|DebugKeyE
  (params (Key :type Key%20Structure) (ActionValue :type Input%20Action%20Value%20Structure))
  (bind _returnvalue (Game|GetPlayerController 0))
  ;[0.05098 0.05098 0.05098] Interact with Starter
  (:Pressed
    (bind _array_element (Utilities|Array|ForEachLoopwithBreak (.TrainerParty (Utilities|Struct|BreakFTrainerPokemon (Variables|/Game/ThirdPerson/Blueprints/BP_ThirdPersonCharacter.BP_ThirdPersonCharacter_C|GetTrainer%20Pokemon (Variables|Default|GetTPC%20Ref)))) :!label _label)
      (:LoopBody
        (if (not (== (.PokemonName (Utilities|Struct|BreakFPokemonPartyInfo _array_element)) ""))
          (Variables|Default|SethasPokemon? true)
          (goto _label Break)))
      (:Completed
        (if (not (Variables|Default|GethasPokemon?))
          (Variables|/Script/Engine.PlayerController|SetbShowMouseCursor _returnvalue true)
          (Input|SetInputModeUIOnly _returnvalue 0 "DoNotLock" false)
          (Pawn|Components|CharacterMovement|SetMovementMode (Variables|/Script/Engine.Character|GetCharacterMovement (Variables|Default|GetTPC%20Ref)) "MOVE_Swimming" 0)
          (bind _returnvalue_2 (Game|ConstructObjectfromClass "/Game/PokemonInfo/PokemonStarter/W_AcceptPokemon.W_AcceptPokemon_C" (Variables|Default|GetPokemon%20Name) (Variables|Default|GetStarterPokemon) (Variables|Default|GetPokeball)))
          (UserInterface|Viewport|AddtoViewport _returnvalue_2 0))))))

(fn ConstructionScript)